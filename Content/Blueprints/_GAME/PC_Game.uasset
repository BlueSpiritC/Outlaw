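; PC_Game is a player controller Blueprint that sets up Enhanced Input for the local player.
; On BeginPlay, a local controller adds the IMC_Input mapping context through the Enhanced Input local player subsystem.
; GetPCBase returns the controller itself, while GetBaseCharacter and GetPlayerCharacterBase are empty getters that return no character.
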(event EventBeginPlay
  (if (Pawn|IsLocalPlayerController)
    ;[0 0 0] Bind Input Mapping Context
    (Input|AddMappingContext (PlayerController|LocalPlayerSubsystems|GetEnhancedInputLocalPlayerSubsystem) "/Game/Blueprints/Player/Input/IMC_Input.IMC_Input" 0 "(bIgnoreAllPressedKeysUntilRelease=True,bForceImmediately=False,bNotifyUserSettings=False)")))

(fn ConstructionScript)

(fn GetBaseCharacter
  (return 0))

(fn GetPCBase
  (return self))

(fn GetPlayerCharacterBase
  (return 0))