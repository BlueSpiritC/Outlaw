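; Anim notify state that blends out its montage while the notify window is ticking.
; On each tick it requires a Character owner and a montage animation, then calls Montage Stop with BlendOutTime.
; A BlendOutCondition switch for unconditional, movement-input or falling blend-out exists but is disconnected, so the stop always happens regardless of that setting.
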(fn ReceivedNotifyTick
  (params (MeshComp :type Skeletal%20Mesh%20Component%20Object%20Reference) (Animation :type Anim%20Sequence%20Base%20Object%20Reference) (FrameDeltaTime :type Float%20%28single-precision%29) (EventReference :type Anim%20Notify%20Event%20Reference%20Structure%20%28by%20ref%29))
  (bind _ascharacter (Utilities|Casting|CastToCharacter (Components|GetOwner MeshComp)))
  (LocalVariables|SetCharacter _ascharacter)
  (LocalVariables|SetAnimInstance (Components|SkeletalMesh|GetAnimInstance MeshComp))
  (bind _asanim_montage (Utilities|Casting|CastToAnimMontage Animation))
  (LocalVariables|SetAnimMontage _asanim_montage)
  (Animation|Montage|MontageStop (LocalVariables|GetAnimInstance) (Variables|Default|GetBlendOutTime) (LocalVariables|GetAnimMontage))
  (return true))