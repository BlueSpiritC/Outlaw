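; Actor component that plays replicated footstep sounds for its owning character.
; Any key press starts a short-delay loop through a server event, which repeats while the pawn has velocity.
; Each pass traces down from both foot sockets, using a DoOnce per foot that resets when the trace misses, so each contact fires once.
; Contacts route through server-to-multicast events that play the sound at the pawn's location.
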(event Custom|CalculateFootstepSFX
  ;[0 0 0] If player is moving, start calling to calculate whether to play footstep sfx or not
  (if (> (Math|Vector|VectorLength (Transformation|GetVelocity (Variables|Default|GetOwnerPawn))) 1.0)
    (Utilities|FlowControl|Sequence
      (:then_0
        (CallFunction|PlayFootstepsSFXFootL)
        (CallFunction|PlayFootstepsSFXFootR))
      (:then_1
        ;;[0 0 0] Loop
        (Utilities|FlowControl|Delay 0.05)
        (CallFunction|SRVCalculateFootstepSFX)))))

(event Custom|SRV_PlayFootstepsSFX_FootR
  ;[0 0 0] Line traces to detect whether play sound or not
  ;;[0.6308 0.008023 0] Server call for multicast event to play sound for each foot
  (CallFunction|MCPlayFootstepsSFXFootR))

(event Custom|PlayFootstepsSFX_FootR
  (bind _ownermesh (Variables|Default|GetOwnerMesh))
  (bind _returnvalue (Transformation|GetSocketLocation _ownermesh "foot_r"))
  ;[0 0 0] Line traces to detect whether play sound or not
  (Utilities|IsValid (Variables|Default|GetOwnerPawn)
    (:Is%20Valid
      (bind _returnvalue_2 (Collision|LineTraceByChannel _returnvalue (- _returnvalue "0.000000,0.000000,15.000000") "TraceTypeQuery1" false 0 "None"))
      (if _returnvalue_2
        (Utilities|FlowControl|DoOnce false :!label _label
          (:Completed
            (CallFunction|SRVPlayFootstepsSFXFootR)))
        (else
          (goto _label Reset))))))

(event Custom|SRV_CalculateFootstepSFX
  ;[0.6308 0.008023 0] Server call for CalculateFootstepSFX
  (CallFunction|CalculateFootstepSFX))

(event Custom|MC_PlayFootstepsSFX_FootR
  ;[0 0 0] Line traces to detect whether play sound or not
  ;;[1 0.1912 0] Multicast call for each foot sound
  (Audio|PlaySoundatLocation (Variables|Default|GetSound) (Transformation|GetActorLocation (Variables|Default|GetOwnerPawn)) "0, 0, 0" 1.0 1.0 0.0 0 0 0 0))

(event Custom|PlayFootstepsSFX_FootL
  (bind _ownermesh (Variables|Default|GetOwnerMesh))
  (bind _returnvalue (Transformation|GetSocketLocation _ownermesh "foot_l"))
  ;[0 0 0] Line traces to detect whether play sound or not
  (Utilities|IsValid (Variables|Default|GetOwnerPawn)
    (:Is%20Valid
      (bind _returnvalue_2 (Collision|LineTraceByChannel _returnvalue (- _returnvalue "0.000000,0.000000,15.000000") "TraceTypeQuery1" false 0 "None"))
      (if _returnvalue_2
        (Utilities|FlowControl|DoOnce false :!label _label
          (:Completed
            (CallFunction|SRVPlayFootstepsSFXFootL)))
        (else
          (goto _label Reset))))))

(event Custom|MC_PlayFootstepsSFX_FootL
  ;[0 0 0] Line traces to detect whether play sound or not
  ;;[1 0.1912 0] Multicast call for each foot sound
  (Audio|PlaySoundatLocation (Variables|Default|GetSound) (Transformation|GetActorLocation (Variables|Default|GetOwnerPawn)) "0, 0, 0" 1.0 1.0 0.0 0 0 0 0))

(event Custom|SRV_PlayFootstepsSFX_FootL
  ;[0 0 0] Line traces to detect whether play sound or not
  ;;[0.6308 0.008023 0] Server call for multicast event to play sound for each foot
  (CallFunction|MCPlayFootstepsSFXFootL))

(event EventBeginPlay
  ;[0 0 0] Assinging on begin play
  (bind _basecharacter (Class|BPIGetReferences|GetBaseCharacter(Message) (Components|GetOwner)))
  (Variables|Default|SetOwnerPawn _basecharacter)
  (Variables|Default|SetOwnerMesh (Variables|/Script/Engine.Character|GetMesh _basecharacter)))

(event Input|KeyboardEvents|AnyKey
  (params (Key :type Key%20Structure))
  ;[0 0 0] Start calling sound event when starting movement
  (:Pressed
    (Utilities|FlowControl|Delay 0.05)
    (Networking|SwitchHasAuthority
      (:Authority
        (CallFunction|CalculateFootstepSFX))
      (:Remote
        (CallFunction|SRVCalculateFootstepSFX)))))